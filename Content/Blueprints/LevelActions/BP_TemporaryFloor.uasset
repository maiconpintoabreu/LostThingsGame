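; BP_TemporaryFloor is a short-lived platform that shakes, then drops and disappears, with its countdown starting at BeginPlay rather than on contact.
; A ShakePlatform timeline offsets the static mesh along Y through MoveComponentTo, feeding world-location values in as the relative target.
; In parallel, a DelayToDestroy wait enables physics on the mesh, and the actor destroys itself a fraction of a second later.
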(event EventBeginPlay
  (bind _staticmesh (Variables|Default|GetStaticMesh))
  (bind _returnvalue (Transformation|GetWorldLocation _staticmesh))
  (Utilities|FlowControl|Sequence
    (:then_0
      (bind _newtrack_0 (Timeline|ShakePlatform Play)
        (:Update
          (Components|MoveComponentTo _staticmesh (Math|Vector|MakeVector (.x _returnvalue) (+ (.y _returnvalue) _newtrack_0) (.z _returnvalue)) "0, 0, 0" false false 0.2 false))
        (:Finished
          (Components|MoveComponentTo 0 (Transformation|GetWorldLocation (Variables|Default|GetStaticMesh)) "0, 0, 0" false false 0.2 false))))
    (:then_1
      (Utilities|FlowControl|Delay (Variables|Default|GetDelayToDestroy))
      (Physics|SetSimulatePhysics (Variables|Default|GetStaticMesh) true)
      (Utilities|FlowControl|Delay 0.2)
      (Actor|DestroyActor))))

(event Collision|EventActorBeginOverlap
  (params (OtherActor :type Actor%20Object%20Reference)))

(event EventTick
  (params (DeltaSeconds :type Float%20%28single-precision%29)))

(fn ConstructionScript)