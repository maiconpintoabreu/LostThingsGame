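; BP_NextLevel is a level-progression actor that shows an intro message and moves the player to the next level.
; On BeginPlay it finds the current level in Levels and briefly shows the matching Mensages entry in a WB_LevelInformation widget.
; When a ThirdPersonCharacter overlaps NextLevelZone, it sets that character's NextLevel flag and opens the following Levels entry.
; The last or an unlisted level leads to "End", with the unlisted case also printing "Congratulations".
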(event OnComponentBeginOverlap(NextLevelZone)
  (params (OverlappedComponent :type Primitive%20Component%20Object%20Reference) (OtherActor :type Actor%20Object%20Reference) (OtherComp :type Primitive%20Component%20Object%20Reference) (OtherBodyIndex :type Integer) (bFromSweep :type Boolean) (SweepResult :type Hit%20Result%20Structure%20%28by%20ref%29))
  (bind _levels (Variables|Default|GetLevels))
  (bind _levels_2 (Variables|Default|GetLevels))
  (bind _asthird_person_character (Utilities|Casting|CastToThirdPersonCharacter OtherActor))
  (Variables|/Game/Blueprints/ThirdPersonCharacter.ThirdPersonCharacter_C|SetNextLevel _asthird_person_character true)
  (bind _returnvalue (Game|GetCurrentLevelName true))
  (if (and (<= (Utilities|Array|FindItem _levels_2 (Utilities|String|StringToName _returnvalue)) (- (Utilities|Array|Length _levels_2) 1)) (!= (Utilities|Array|FindItem _levels_2 (Utilities|String|StringToName _returnvalue)) -1))
    (if (Utilities|Array|IsValidIndex _levels (+ (Utilities|Array|FindItem _levels_2 (Utilities|String|StringToName _returnvalue)) 1))
      (Game|OpenLevel(byName) (Utilities|Array|Get(acopy) _levels (+ (Utilities|Array|FindItem _levels_2 (Utilities|String|StringToName _returnvalue)) 1)))
      (else
        (Game|OpenLevel(byName) "End" :!label _label)))
    (else
      (Development|PrintString "Congratulations")
      (goto _label))))

(event EventBeginPlay
  (bind _levels (Variables|Default|GetLevels))
  (bind _returnvalue (Game|GetCurrentLevelName true))
  (if (and (<= (Utilities|Array|FindItem _levels (Utilities|String|StringToName _returnvalue)) (- (Utilities|Array|Length _levels) 1)) (!= (Utilities|Array|FindItem _levels (Utilities|String|StringToName _returnvalue)) -1))
    (bind _returnvalue_2 (UserInterface|CreateWidget "/Game/UI/WB_LevelInformation.WB_LevelInformation_C" 0 (Utilities|Array|Get(acopy) (Variables|Default|GetMensages) (Utilities|Array|FindItem _levels (Utilities|String|StringToName _returnvalue)))))
    (UserInterface|Viewport|AddtoViewport _returnvalue_2 0)
    (Utilities|FlowControl|Delay 2.0)
    (Widget|RemovefromParent _returnvalue_2)))

(event Collision|EventActorBeginOverlap
  (params (OtherActor :type Actor%20Object%20Reference)))

(event EventTick
  (params (DeltaSeconds :type Float%20%28single-precision%29)))

(fn ConstructionScript)