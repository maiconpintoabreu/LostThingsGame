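; BP_Run is a gameplay ability that makes the player's ThirdPersonCharacter run temporarily.
; Activation commits the ability, calls Run on player character 0, then calls StopRunning after a two-second delay, without calling EndAbility.
; The end-ability event also calls StopRunning before passing to the parent.
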(event Ability|EventActivateAbility
  (Ability|CommitAbility)
  (bind _asthird_person_character (Utilities|Casting|CastToThirdPersonCharacter (Game|GetPlayerCharacter 0)))
  (Default|Run _asthird_person_character)
  (Utilities|FlowControl|Delay 2.0)
  (Default|StopRunning _asthird_person_character))

(event Ability|EventOnEndAbility
  (params (bWasCancelled :type Boolean))
  (bind _asthird_person_character (Utilities|Casting|CastToThirdPersonCharacter (Game|GetPlayerCharacter 0)))
  (Default|StopRunning _asthird_person_character)
  (|CallParentFunction bWasCancelled))