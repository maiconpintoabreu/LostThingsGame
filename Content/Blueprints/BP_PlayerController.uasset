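; Player controller Blueprint that can add a mobile HUD widget to the viewport on Android.
; ShowHUD checks the platform name, creates and caches WB_HUD_Mobile if none is valid, then adds it to the viewport.
; BeginPlay's branch condition is fixed at true, so its ShowHUD call on the false path never runs.
; The level-name check for Intro and End is left unconnected.
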(event Custom|ShowHUD
  (if (Utilities|Enum|Equal(Enum) (Game|GetPlatformName) "Android")
    (Utilities|IsValid (Variables|Default|GetMobileHUD)
      (:Is%20Valid
        _)
      (:Is%20Not%20Valid
        (bind _returnvalue (UserInterface|CreateWidget "/Game/UI/WB_HUD_Mobile.WB_HUD_Mobile_C"))
        (Variables|Default|SetMobileHUD _returnvalue)))
    (UserInterface|Viewport|AddtoViewport (Variables|Default|GetMobileHUD) 0)))

(event EventBeginPlay
  (bind _returnvalue (Game|GetCurrentLevelName true))
  (if (not true)
    (CallFunction|ShowHUD)))

(event EventTick
  (params (DeltaSeconds :type Float%20%28single-precision%29)))

(fn ConstructionScript)