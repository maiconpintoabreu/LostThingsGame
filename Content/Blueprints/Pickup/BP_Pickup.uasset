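; BP_Pickup is a world pickup that displays a data-driven item and shows an action prompt when the player is near.
; On BeginPlay it resolves the item's primary asset ID and creates a hidden WB_PickupAction widget for it.
; For lost items, it briefly spawns the equip class to copy its mesh, then destroys it.
; Sphere overlaps with ThirdPersonCharacter toggle the widget; collection is not handled here.
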(event OnComponentBeginOverlap(Sphere)
  (params (OverlappedComponent :type Primitive%20Component%20Object%20Reference) (OtherActor :type Actor%20Object%20Reference) (OtherComp :type Primitive%20Component%20Object%20Reference) (OtherBodyIndex :type Integer) (bFromSweep :type Boolean) (SweepResult :type Hit%20Result%20Structure%20%28by%20ref%29))
  (Utilities|Casting|CastToThirdPersonCharacter OtherActor)
  (Rendering|SetVisibility (Variables|Default|GetWidget) true false))

(event OnComponentEndOverlap(Sphere)
  (params (OverlappedComponent :type Primitive%20Component%20Object%20Reference) (OtherActor :type Actor%20Object%20Reference) (OtherComp :type Primitive%20Component%20Object%20Reference) (OtherBodyIndex :type Integer))
  (Utilities|Casting|CastToThirdPersonCharacter OtherActor)
  (Rendering|SetVisibility (Variables|Default|GetWidget) false false))

(event EventBeginPlay
  (bind _widget (Variables|Default|GetWidget))
  (bind _asfsitem (Utilities|Casting|CastToFSItem (Class|KismetSystemLibrary|GetObjectfromPrimaryAssetId (Variables|Default|GetItemFromDataset)))
    (:then
      (bind _output_get (Variables|Default|SetItemLoaded _asfsitem))
      (bind _returnvalue (UserInterface|CreateWidget "/Game/UI/WB_PickupAction.WB_PickupAction_C" 0 _output_get))
      (UserInterface|SetWidget _widget _returnvalue)
      (Rendering|SetVisibility _widget false false)
      (bind _asfslost_item (Utilities|Casting|CastToFSLostItem (Variables|Default|GetItemLoaded)))
      (bind _returnvalue_2 (Game|SpawnActorfromClass (Variables|/Script/GGJLostThings.FSEquipItem|GetEquipClass _asfslost_item) (Math|Conversions|ToTransform(Vector) (Transformation|GetWorldLocation (Variables|Default|GetStaticMesh))) "Undefined" 0 0))
      (bind _asbp_lost_items (Utilities|Casting|CastToBP_LostItems _returnvalue_2))
      (bind _staticmesh (Default|GetMesh _asbp_lost_items))
      (Components|StaticMesh|SetStaticMesh (Variables|Default|GetStaticMesh) _staticmesh)
      (Actor|DestroyActor _returnvalue_2))
    (:CastFailed
      (Development|PrintString "Error to load item"))))

(fn ConstructionScript)